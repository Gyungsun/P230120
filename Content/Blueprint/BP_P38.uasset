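; BP_P38 is a twin-propeller P-38 aircraft that flies forward on its own.
; Each Tick it spins both propellers around local roll by RotateSpeed and moves the actor along local X by MoveSpeed, both scaled by delta time.
; Input is not wired to flight: the pitch axis only prints its value and Roll is empty.
; NewFunction offsets the actor along world X but is not called in these graphs.
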(event EventTick
  (params (DeltaSeconds :type Float%20%28single-precision%29))
  ;[1 1 1] Rotate Right Propeller
  (Transformation|AddLocalRotation (Variables|Default|GetPropellerRight) (Math|Rotator|MakeRotator (* (Utilities|Time|GetWorldDeltaSeconds) (Variables|속력|GetRotateSpeed)) 0.0 0.0) false false)
  ;[1 1 1] Rotate Left Propeller
  (Transformation|AddLocalRotation (Variables|Default|GetPropellerLft) (Math|Rotator|MakeRotator (* (Utilities|Time|GetWorldDeltaSeconds) (Variables|속력|GetRotateSpeed)) 0.0 0.0) false false)
  ;[1 1 1] AirPlain go Forward
  (Transformation|AddActorLocalOffset self (Math|Vector|MakeVector (* (Utilities|Time|GetWorldDeltaSeconds) (Variables|속력|GetMoveSpeed)) 0.0 0.0) false false))

(event Input|ActionEvents|InputActionFire
  (params (Key :type Key%20Structure :default "None")))

(event Input|AxisEvents|InputAxispitch
  (params (AxisValue :type Float%20%28single-precision%29))
  (Development|PrintString (Utilities|String|ToString(Float) AxisValue)))

(event Input|AxisEvents|InputAxisRoll
  (params (AxisValue :type Float%20%28single-precision%29)))

(fn ConstructionScript)

(fn NewFunction
  (params (who :type Actor%20Component%20Object%20Reference))
  (Transformation|AddActorWorldOffset (Math|Vector|MakeVector (* (Utilities|Time|GetWorldDeltaSeconds) (Variables|속력|GetMoveSpeed)) 0.0 0.0)))