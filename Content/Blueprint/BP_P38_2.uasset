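; P38 airplane pawn controlled by pitch and roll input, firing rockets on the Fire action.
; Tick spins both propellers, scaled by delta time, and calls AddMovementInput with a zero direction, so that call gives no thrust.
; Axis inputs feed controller pitch and roll, while Fire spawns BP_Rocket at the Arrow's transform.
; Manual rotate and forward-offset nodes are disconnected; NewFunction, a world-X offset, is never called here.
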(event EventTick
  (params (DeltaSeconds :type Float%20%28single-precision%29))
  ;[1 1 1] Rotate Right Propeller
  (Transformation|AddLocalRotation (Variables|Default|GetPropellerRight) (Math|Rotator|MakeRotator (* (Utilities|Time|GetWorldDeltaSeconds) (Variables|속력|GetPropellerRotateSpeed)) 0.0 0.0) false false)
  ;[1 1 1] Rotate Left Propeller
  (Transformation|AddLocalRotation (Variables|Default|GetPropellerLft) (Math|Rotator|MakeRotator (* (Utilities|Time|GetWorldDeltaSeconds) (Variables|속력|GetPropellerRotateSpeed)) 0.0 0.0) false false)
  ;[1 1 1] Movement 이동
  (Pawn|Input|AddMovementInput "0, 0, 0" 0.5 false))

(event Input|ActionEvents|InputActionFire
  (params (Key :type Key%20Structure :default "None"))
  (:Pressed
    (Game|SpawnActorfromClass "/Game/Blueprint/BP_Rocket.BP_Rocket_C" (Transformation|GetWorldTransform (Variables|Default|GetArrow)) "AdjustIfPossibleButAlwaysSpawn" 0 0)))

(event Input|AxisEvents|InputAxispitch
  (params (AxisValue :type Float%20%28single-precision%29))
  (Pawn|Input|AddControllerPitchInput AxisValue))

(event Input|AxisEvents|InputAxisRoll
  (params (AxisValue :type Float%20%28single-precision%29))
  (Pawn|Input|AddControllerRollInput AxisValue))

(fn ConstructionScript)

(fn NewFunction
  (params (who :type Actor%20Component%20Object%20Reference))
  (Transformation|AddActorWorldOffset (Math|Vector|MakeVector (* (Utilities|Time|GetWorldDeltaSeconds) (Variables|속력|GetMoveSpeed)) 0.0 0.0)))